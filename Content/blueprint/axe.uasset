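; Axe actor that continuously spins its Cube mesh and reacts when a ThirdPersonCharacter enters or leaves its Box trigger.
; A self-restarting delay loop advances the pitch angle, while overlaps change a Y offset arithmetically and each entry bumps a material index.
; RepNotify functions apply rotation and location to Cube, and cycle five materials in staggered order across the cubes and the referenced Floor.
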(event OnComponentBeginOverlap(Box)
  (params (OverlappedComponent :type Primitive%20Component%20Object%20Reference) (OtherActor :type Actor%20Object%20Reference) (OtherComp :type Primitive%20Component%20Object%20Reference) (OtherBodyIndex :type Integer) (bFromSweep :type Boolean) (SweepResult :type Hit%20Result%20Structure%20%28by%20ref%29))
  (Utilities|Casting|CastToThirdPersonCharacter OtherActor)
  (bind _result (Math|Float|IncrementFloat (Variables|Default|GetNew%20Location%20Y))
    (:%20%20
      (Variables|Default|SetNew%20Location%20Y (* _result _result))
      (Variables|Default|Setmatsetindex (+ (Variables|Default|Getmatsetindex) 1)))))

(event OnComponentEndOverlap(Box)
  (params (OverlappedComponent :type Primitive%20Component%20Object%20Reference) (OtherActor :type Actor%20Object%20Reference) (OtherComp :type Primitive%20Component%20Object%20Reference) (OtherBodyIndex :type Integer))
  (Utilities|Casting|CastToThirdPersonCharacter OtherActor)
  (Variables|Default|SetNew%20Location%20Y (* (- (Variables|Default|GetNew%20Location%20Y) 1.0) (Variables|Default|GetNew%20Location%20Y))))

(event Custom|rotate
  (Variables|Default|Setadder (Math|Float|%(Float) (+ (Variables|Default|Getadder) 0.2) 3.6e+02))
  (Utilities|FlowControl|Delay 0.04)
  (CallFunction|Rotate))

(event EventBeginPlay
  (CallFunction|Rotate))

(event Collision|EventActorBeginOverlap
  (params (OtherActor :type Actor%20Object%20Reference)))

(event EventTick
  (params (DeltaSeconds :type Float%20%28single-precision%29)))

(fn ConstructionScript)

(fn OnRepAdder
  (Transformation|SetRelativeRotation (Variables|Default|GetCube) (Math|Rotator|MakeRotator 0.0 (Variables|Default|Getadder) 0.0) false true))

(fn OnRepNewLocationY
  (Transformation|SetRelativeLocation (Variables|Default|GetCube) (Math|Vector|MakeVector 0.0 (Variables|Default|GetNew%20Location%20Y) 0.0) false false))

(fn OnRepMatsetindex
  (bind _matsetindex (Variables|Default|Getmatsetindex))
  (bind _returnvalue (+ _matsetindex 1))
  (bind _returnvalue_2 (+ _returnvalue 1))
  (bind _returnvalue_3 (+ _returnvalue_2 1))
  (Rendering|Material|SetMaterial (Variables|Default|GetCube) 0 (Utilities|Array|Get(acopy) (Variables|Default|GetMaterial) (Math|Integer|%(Integer) _matsetindex 5)))
  (Rendering|Material|SetMaterial (Variables|Default|GetCube1) 0 (Utilities|Array|Get(acopy) (Variables|Default|GetMaterial) (Math|Integer|%(Integer) _returnvalue 5)))
  (Rendering|Material|SetMaterial (Variables|Default|GetCube2) 0 (Utilities|Array|Get(acopy) (Variables|Default|GetMaterial) (Math|Integer|%(Integer) _returnvalue_2 5)))
  (Rendering|Material|SetMaterial (Variables|Default|GetCube3) 0 (Utilities|Array|Get(acopy) (Variables|Default|GetMaterial) (Math|Integer|%(Integer) _returnvalue_3 5)))
  (Rendering|Material|SetMaterial (Variables|Default|GetCube4) 0 (Utilities|Array|Get(acopy) (Variables|Default|GetMaterial) (Math|Integer|%(Integer) (+ _returnvalue_3 1) 5))))